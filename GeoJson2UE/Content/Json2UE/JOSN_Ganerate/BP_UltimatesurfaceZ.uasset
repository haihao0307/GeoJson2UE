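; Blueprint actor that turns GeoJSON polygon features from MeshJson into Cesium-georeferenced surface actors.
; The jsonArray event destroys previous surfaces, then parses the JSON with VaRest.
; It converts each feature's longitude/latitude coordinates to Unreal XY through CesiumGeoreference at a fixed height, flattening all rings into one vertex list.
; Each feature spawns an attached BP_SurfaceOutPutZ with those vertices and a randomly suffixed name.
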(event `jsonArray`
  (bind _meshactorarray (`self.meshActorArray`))
  (for _array_element _meshactorarray
    (`self.K2_DestroyActor` _array_element))
  (`KismetArrayLibrary.Array_Clear` _meshactorarray)
  (bind _returnvalue (`VaRestSubsystem.ConstructVaRestJsonObject` (subsystem `VaRestSubsystem`)))
  (`VaRestJsonObject.DecodeJson` _returnvalue (`self.meshJson`) true)
  (for _array_element_2 (`VaRestJsonObject.GetObjectArrayField` _returnvalue "features")
    (for _array_element_3 (`VaRestJsonObject.GetArrayField` (`VaRestJsonObject.GetObjectField` _array_element_2 "geometry") "coordinates")
      (for _array_element_4 (`VaRestJsonValue.AsArray` _array_element_3)
        (bind _returnvalue_2 (`GameplayStatics.GetActorOfClass` "/Script/CesiumRuntime.CesiumGeoreference"))
        (bind _returnvalue_3 (`VaRestJsonValue.AsArray` _array_element_4))
        (bind (_returnvalue_x _returnvalue_y) (`KismetMathLibrary.BreakVector` (`CesiumGeoreference.TransformLongitudeLatitudeHeightPositionToUnreal` _returnvalue_2 (`KismetMathLibrary.MakeVector` (`VaRestJsonValue.AsNumber` (`|GetArrayItem` _returnvalue_3)) (`VaRestJsonValue.AsNumber` (`|GetArrayItem` _returnvalue_3 1)) 100.0))))
        (`KismetArrayLibrary.Array_Add` (`self.Polygon Vertices`) (`KismetMathLibrary.MakeVector2D` _returnvalue_x _returnvalue_y))))
    (bind _returnvalue_4 (`|SpawnActorFromClass` "/GeoJson2UE/demo/blueptint/BP_SurfaceOutPutZ.BP_SurfaceOutPutZ_C" (`KismetMathLibrary.MakeTransform` (0.0 0.0 0.0)) "Undefined" "MultiplyWithRoot" null (`self.Polygon Vertices`) (`KismetStringLibrary.Concat_StrStr` (`VaRestJsonObject.GetStringField` (`VaRestJsonObject.GetObjectField` _array_element_2 "properties") "name") "_" (`KismetStringLibrary.Conv_IntToString` (`KismetMathLibrary.RandomInteger` 999))) null))
    (`KismetArrayLibrary.Array_Add` (`self.meshActorArray`))
    (`self.K2_AttachToActor` _returnvalue_4 self "None" "KeepWorld" "KeepWorld" "KeepWorld" true)
    (`KismetArrayLibrary.Array_Clear` (`self.Polygon Vertices`))))

(fn `UserConstructionScript`)