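; Actor that builds spline output actors in the world from GeoJSON-style line features stored in MeshJson.
; Its jsonArray event destroys previously spawned lines, then parses the features with VaRest.
; Each longitude/latitude/height coordinate converts to Unreal space through CesiumGeoreference, filling 2D and 3D point arrays.
; Every feature spawns an attached BP_SplineOutPut with those points and a name plus random suffix, tracked in LineArray.
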(event `jsonArray`
  (bind _linearray (`self.lineArray`))
  (bind _z (.z (`self.K2_GetActorLocation`)))
  (`KismetArrayLibrary.Array_Clear` (`self.Polygon Vertices`))
  (for _array_element _linearray
    (`self.K2_DestroyActor` _array_element))
  (`KismetArrayLibrary.Array_Clear` _linearray)
  (bind _returnvalue (`VaRestSubsystem.ConstructVaRestJsonObject` (subsystem `VaRestSubsystem`)))
  (`VaRestJsonObject.DecodeJson` _returnvalue (`self.meshJson`) true)
  (for _array_element_2 (`VaRestJsonObject.GetObjectArrayField` _returnvalue "features")
    (for _array_element_3 (`VaRestJsonObject.GetArrayField` (`VaRestJsonObject.GetObjectField` _array_element_2 "geometry") "coordinates")
      (bind _returnvalue_2 (`GameplayStatics.GetActorOfClass` "/Script/CesiumRuntime.CesiumGeoreference"))
      (bind _returnvalue_3 (`VaRestJsonValue.AsArray` _array_element_3))
      (bind _returnvalue_4 (`VaRestJsonValue.AsNumber` (`|GetArrayItem` _returnvalue_3 2)))
      (bind (_returnvalue_x _returnvalue_y _returnvalue_z) (`KismetMathLibrary.BreakVector` (`CesiumGeoreference.TransformLongitudeLatitudeHeightPositionToUnreal` _returnvalue_2 (`KismetMathLibrary.MakeVector` (`VaRestJsonValue.AsNumber` (`|GetArrayItem` _returnvalue_3)) (`VaRestJsonValue.AsNumber` (`|GetArrayItem` _returnvalue_3 1)) _returnvalue_4))))
      (`KismetArrayLibrary.Array_Add` (`self.Polygon Vertices`) (`KismetMathLibrary.MakeVector2D` _returnvalue_x _returnvalue_y))
      (`KismetArrayLibrary.Array_Add` (`self.Array`) (`KismetMathLibrary.MakeVector` _returnvalue_x _returnvalue_y _returnvalue_z))
      (`KismetSystemLibrary.PrintString` (`KismetStringLibrary.Conv_DoubleToString` _returnvalue_4)))
    (bind _returnvalue_5 (`|SpawnActorFromClass` "/GeoJson2UE/demo/blueptint/line/BP_SplineOutPut.BP_SplineOutPut_C" (`KismetMathLibrary.MakeTransform` (`KismetMathLibrary.MakeVector` 0.0 0.0 _z)) "Undefined" "MultiplyWithRoot" null (`self.Polygon Vertices`) (`KismetStringLibrary.Concat_StrStr` (`VaRestJsonObject.GetStringField` (`VaRestJsonObject.GetObjectField` _array_element_2 "properties") "name") "_" (`KismetStringLibrary.Conv_IntToString` (`KismetMathLibrary.RandomInteger` 999))) _z self (`self.Array`) null))
    (`KismetArrayLibrary.Array_Add` (`self.lineArray`) _returnvalue_5)
    (`self.K2_AttachToActor` _returnvalue_5 self "None" "KeepWorld" "KeepWorld" "KeepWorld" true)
    (`KismetArrayLibrary.Array_Clear` (`self.Polygon Vertices`))
    (`KismetArrayLibrary.Array_Clear` (`self.Array`))))

(fn `UserConstructionScript`)