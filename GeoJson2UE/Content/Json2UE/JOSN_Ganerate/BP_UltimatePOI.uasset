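; Spawns a named BP_POI marker for each point feature in a GeoJSON string, placed on the Cesium globe.
; The jsonArray event destroys previously spawned markers, then parses MeshJson with VaRest.
; It converts each feature's longitude, latitude and height to Unreal space through CesiumGeoreference.
; Each marker gets the feature's name, is attached to this actor and is tracked in LineArray for cleanup.
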(event `jsonArray`
  (bind _linearray (`self.lineArray`))
  (`KismetArrayLibrary.Array_Clear` (`self.Polygon Vertices`))
  (for _array_element _linearray
    (`self.K2_DestroyActor` _array_element))
  (`KismetArrayLibrary.Array_Clear` _linearray)
  (bind _returnvalue (`VaRestSubsystem.ConstructVaRestJsonObject` (subsystem `VaRestSubsystem`)))
  (`VaRestJsonObject.DecodeJson` _returnvalue (`self.meshJson`) true)
  (for _array_element_2 (`VaRestJsonObject.GetObjectArrayField` _returnvalue "features")
    (bind _returnvalue_2 (`GameplayStatics.GetActorOfClass` "/Script/CesiumRuntime.CesiumGeoreference"))
    (bind _returnvalue_3 (`VaRestJsonObject.GetArrayField` (`VaRestJsonObject.GetObjectField` _array_element_2 "geometry") "coordinates"))
    (set `self.Spawn Transform Location` (`CesiumGeoreference.TransformLongitudeLatitudeHeightPositionToUnreal` _returnvalue_2 (`KismetMathLibrary.MakeVector` (`VaRestJsonValue.AsNumber` (`|GetArrayItem` _returnvalue_3)) (`VaRestJsonValue.AsNumber` (`|GetArrayItem` _returnvalue_3 1)) (`VaRestJsonValue.AsNumber` (`|GetArrayItem` _returnvalue_3 2)))))
    (bind _returnvalue_4 (`VaRestJsonObject.GetStringField` (`VaRestJsonObject.GetObjectField` _array_element_2 "properties") "name"))
    (`KismetSystemLibrary.PrintString` _returnvalue_4)
    (bind _returnvalue_5 (`|SpawnActorFromClass` "/GeoJson2UE/demo/blueptint/line/BP_POI.BP_POI_C" (`KismetMathLibrary.MakeTransform` (`self.Spawn Transform Location`)) "Undefined" "MultiplyWithRoot" null _returnvalue_4 null))
    (`KismetArrayLibrary.Array_Add` (`self.lineArray`) _returnvalue_5)
    (`self.K2_AttachToActor` _returnvalue_5 self "None" "KeepWorld" "KeepWorld" "KeepWorld" true)))

(fn `UserConstructionScript`)